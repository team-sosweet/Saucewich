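; Pickup spawner actor that carries a widget component showing a spawn HUD; the graph contains no spawning logic.
; On BeginPlay it initializes the HUD widget with itself and caches player 0's controlled pawn.
; Every Tick it maps its distance to that pawn onto the widget's square draw size, shrinking the HUD as the player moves away, within clamped limits.
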(event EventTick
  (params (DeltaSeconds :type Float%20%28single-precision%29))
  (bind _returnvalue (Transformation|GetActorLocation))
  (bind _local_pawn (Variables|Default|GetLocal%20Pawn))
  (bind _returnvalue_2 (Transformation|GetActorLocation _local_pawn))
  (bind _returnvalue_3 (Math|Vector|Distance(Vector) _returnvalue _returnvalue_2))
  (bind _returnvalue_4 (Math|Float|MapRangeClamped _returnvalue_3 0.0 2e+03 1.2e+02 4e+01))
  (Class|WidgetComponent|SetDrawSize (Variables|컴포넌트|GetWidget) (Math|Vector2D|MakeVector2D _returnvalue_4 _returnvalue_4)))

(event EventBeginPlay
  (bind _asumg_spawn_hud (Utilities|Casting|CastToUMG_SpawnHUD (UserInterface|GetUserWidgetObject (Variables|컴포넌트|GetWidget))))
  (Default|Init _asumg_spawn_hud self)
  (Variables|Default|SetLocal%20Pawn (Pawn|GetControlledPawn (Game|GetPlayerController 0))))

(fn ConstructionScript)