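; Online game state Blueprint that prints an on-screen kill message when a player dies.
; On BeginPlay it binds PrintKillLog to the OnPlayerDeath dispatcher, which supplies victim, attacker and inflictor.
; The handler requires all three to be valid and the inflictor to be a Weapon, then formats and briefly prints the message.
; Both the victim and attacker fields use the victim's player name.
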(event Custom|PrintKillLog
  (params (Victim :type Saucewich%20Player%20State%20Object%20Reference) (Attacker :type Saucewich%20Player%20State%20Object%20Reference) (Inflictor :type Actor%20Object%20Reference))
  (if (Math|Boolean|ANDBoolean (Utilities|IsValid Victim) (Utilities|IsValid Attacker) (Utilities|IsValid Inflictor))
    (bind _asweapon (Utilities|Casting|CastToWeapon Inflictor))
    (Development|PrintText (Utilities|Text|FormatText "{victim} was killed with {inflictor} by {attacker}" (Utilities|Text|ToText(String) (PlayerState|GetPlayerName Victim)) (Utilities|Text|ToText(String) (PlayerState|GetPlayerName Victim)) (Variables|/Script/Saucewich.Weapon|GetName _asweapon)) true true "(R=0.000000,G=0.660000,B=1.000000,A=1.000000)" 5.0)))

(event EventBeginPlay
  (EventDispatchers|AssignOnPlayerDeath (delegate Custom|PrintKillLog)))

(fn ConstructionScript)