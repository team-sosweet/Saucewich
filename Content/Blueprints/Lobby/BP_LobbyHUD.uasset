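; BP_LobbyHUD is the lobby HUD, which creates the UMG_Lobby widget for the owning player and adds it to the viewport on BeginPlay.
; CreateMenuWidgets takes a map of buttons to menu widget classes and passes each pair to CreateMenuWidget.
; CreateMenuWidget instantiates the menu, stores it in Menus without displaying it, and binds an event to the button's click.
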(event Custom|Create%20Menu%20Widgets
  (params (Button%20Widget%20Map :type Map%20of%20Button%20Object%20References%20to%20Classs))
  (bind _keys (Utilities|Map|Keys Button%20Widget%20Map))
  (bind _values (Utilities|Map|Values Button%20Widget%20Map))
  (for (_array_element _array_index) _keys
    (CallFunction|CreateMenuWidget (Utilities|Array|Get(acopy) _values _array_index) _array_element)))

(event Custom|Create%20Menu%20Widget
  (params (Menu%20Class :type UMG%20Menu%20Widget%20Class%20Reference) (Button :type Button%20Object%20Reference))
  (bind _returnvalue (UserInterface|CreateWidget Menu%20Class (Game|Player|GetOwningPlayerController)))
  (EventDispatchers|BindEventtoOnClicked Button (EventDispatchers|CreateEvent _returnvalue :!event OnOpen))
  (Utilities|Array|Add (Variables|Default|GetMenus) _returnvalue))

(event EventBeginPlay
  (bind _returnvalue (UserInterface|CreateWidget "/Game/Blueprints/Widget/Lobby/UMG_Lobby.UMG_Lobby_C" (Game|Player|GetOwningPlayerController)))
  (UserInterface|Viewport|AddtoViewport _returnvalue 0))

(fn ConstructionScript)