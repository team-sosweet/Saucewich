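; Player controller for the entry stage that connects the player to a game server and displays error messages.
; JoinGame opens a hardcoded IP address as an absolute level travel, passing the stored player name as a URL option.
; ShowError casts the current HUD to BaseHUD and forwards the message as a non-critical error.
; An unconnected random word pick is left in the event graph.
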(event Custom|ShowError
  (params (Message :type Text))
  (bind _asbase_hud (Utilities|Casting|CastToBaseHUD (HUD|GetHUD)))
  (Class|BaseHUD|ShowError _asbase_hud Message false))

(event Custom|JoinGame
  (Game|OpenLevel(byName) "192.168.137.1" true (Utilities|String|Append "PlayerName=" (Variables|/Script/Saucewich.UserSettings|GetPlayerName (Class|UserSettings|Get)))))

(fn ConstructionScript)