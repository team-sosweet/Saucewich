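; Entry-screen HUD that shows the entry UI and reports any network error left from a previous connection.
; On BeginPlay it creates UMG_Entry, adds it to the viewport, then pops a stored network error from SaucewichInstance.
; If one exists, it calls ShowError with a message selected by failure type.
; Connection lost and timeout get friendly Korean text, while other types show the raw type and message.
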(event EventBeginPlay
  (bind _returnvalue (UserInterface|CreateWidget "/Game/Blueprints/Widget/Lobby/UMG_Entry.UMG_Entry_C" (Game|Player|GetOwningPlayerController)))
  (bind _output_get (Variables|Default|SetUMG_Entry _returnvalue))
  (UserInterface|Viewport|AddtoViewport _output_get 0)
  (bind (_type _msg _returnvalue_2) (Class|SaucewichInstance|PopNetworkError (.AsSaucewich%20Instance (Utilities|Casting|CastToSaucewichInstance (Game|GetGameInstance)))))
  (if _returnvalue_2
    (Class|BaseHUD|ShowError (Utilities|Select :Index _type :NetDriverAlreadyExists (Utilities|Text|FormatText "{0} 
{1}" (Utilities|Text|ToText(String) (Utilities|String|EnumtoString _type)) (Utilities|Text|ToText(String) _msg)) :NetDriverCreateFailure (Utilities|Text|FormatText "{0} 
{1}" (Utilities|Text|ToText(String) (Utilities|String|EnumtoString _type)) (Utilities|Text|ToText(String) _msg)) :NetDriverListenFailure (Utilities|Text|FormatText "{0} 
{1}" (Utilities|Text|ToText(String) (Utilities|String|EnumtoString _type)) (Utilities|Text|ToText(String) _msg)) :ConnectionLost "오랜 시간 입력이 없어 연결이 끊어졌습니다." :ConnectionTimeout "인터넷 연결을 확인해주세요." :FailureReceived (Utilities|Text|FormatText "{0} 
{1}" (Utilities|Text|ToText(String) (Utilities|String|EnumtoString _type)) (Utilities|Text|ToText(String) _msg)) :OutdatedClient (Utilities|Text|FormatText "{0} 
{1}" (Utilities|Text|ToText(String) (Utilities|String|EnumtoString _type)) (Utilities|Text|ToText(String) _msg)) :OutdatedServer (Utilities|Text|FormatText "{0} 
{1}" (Utilities|Text|ToText(String) (Utilities|String|EnumtoString _type)) (Utilities|Text|ToText(String) _msg)) :PendingConnectionFailure (Utilities|Text|FormatText "{0} 
{1}" (Utilities|Text|ToText(String) (Utilities|String|EnumtoString _type)) (Utilities|Text|ToText(String) _msg)) :NetGuidMismatch (Utilities|Text|FormatText "{0} 
{1}" (Utilities|Text|ToText(String) (Utilities|String|EnumtoString _type)) (Utilities|Text|ToText(String) _msg)) :NetChecksumMismatch (Utilities|Text|FormatText "{0} 
{1}" (Utilities|Text|ToText(String) (Utilities|String|EnumtoString _type)) (Utilities|Text|ToText(String) _msg))))))

(fn ConstructionScript)