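; BP_RandomIngredientBox is a pickup box in the MakeSandwich game mode that gives a random sandwich ingredient to whoever picks it up.
; On pickup, it reads the SandwichIngredients collection from the game state, converts it to an array and picks a random entry.
; It passes that entry to PickupIngredient on the picker's MakeSandwichPlayerState, and does nothing if either state cast fails.
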(event EventOnPickedUp
  (params (By :type Tps%20Character%20Object%20Reference))
  (bind _asmake_sandwich_player_state (Utilities|Casting|CastToMakeSandwichPlayerState (Variables|/Script/Engine.Pawn|GetPlayerState By)))
  (bind _asmake_sandwich_state (Utilities|Casting|CastToMakeSandwichState (Game|GetGameState)))
  (bind _result (Utilities|Set|ToArray (Variables|/Script/Saucewich.MakeSandwichState|GetSandwichIngredients _asmake_sandwich_state)))
  (Class|MakeSandwichPlayerState|PickupIngredient _asmake_sandwich_player_state (Utilities|Array|Get(acopy) _result (Math|Random|RandomInteger (Utilities|Set|Length (Variables|/Script/Saucewich.MakeSandwichState|GetSandwichIngredients _asmake_sandwich_state))))))

(fn ConstructionScript
  (|CallParentFunction))