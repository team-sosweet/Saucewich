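; BP_Perk is a pickup entity in the MakeSandwich game mode that grants its perk to the picker's whole team.
; When picked up, the authority gets all players on that team from the Saucewich game state and adds this perk's class to each one's TpsCharacter pawn.
; An eating sound is also spawned attached to the character that picked it up.
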(event EventOnPickedUp
  (params (By :type Tps%20Character%20Object%20Reference))
  (Utilities|FlowControl|Sequence
    (:then_0
      (Networking|SwitchHasAuthority
        (:Authority
          (bind _assaucewich_game_state (Utilities|Casting|CastToSaucewichGameState (Game|GetGameState)))
          (for _array_element (Class|SaucewichGameState|GetPlayersbyTeam _assaucewich_game_state (Class|TpsCharacter|GetTeam By))
            (bind _astps_character (Utilities|Casting|CastToTpsCharacter (Variables|/Script/Engine.PlayerState|GetPawnPrivate _array_element)))
            (Class|TpsCharacter|AddPerk _astps_character (Utilities|GetClass self))))))
    (:then_1
      (Audio|SpawnSoundAttached "/Game/Assets/Sound/eat.eat" (Variables|/Script/Engine.Actor|GetRootComponent By) "None" "0, 0, 0" "0, 0, 0" "KeepRelativeOffset" false 1.0 1.0 0.0 0 0))))

(fn ConstructionScript)