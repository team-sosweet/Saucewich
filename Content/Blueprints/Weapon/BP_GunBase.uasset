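; BP_GunBase is a gun Blueprint whose Shoot event fires a projectile toward what the player's camera is looking at.
; Shoot traces from the camera using the Projectile profile with debug drawing, and runs only when a player-controlled pawn owns the gun.
; It spawns a scaled-down BP_Projectile at the Muzzle socket, rotated toward the hit point, or using the socket's rotation when nothing is hit.
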(event EventShoot
  (bind _mesh (Variables|Character|GetMesh))
  (bind _returnvalue (Transformation|GetSocketLocation _mesh "Muzzle"))
  (bind _aspawn (Utilities|Casting|CastToPawn (Components|GetOwner)))
  (bind _asplayer_controller (Utilities|Casting|CastToPlayerController (Pawn|GetController _aspawn)))
  (bind (_outhit _returnvalue_2) (Class|KismetSystemLibrary|LineTraceSinglebyProfile (Camera|GetCameraLocation (Variables|/Script/Engine.PlayerController|GetPlayerCameraManager _asplayer_controller)) (+ (Camera|GetCameraLocation (Variables|/Script/Engine.PlayerController|GetPlayerCameraManager _asplayer_controller)) (* (Transformation|GetActorForwardVector (Variables|/Script/Engine.PlayerController|GetPlayerCameraManager _asplayer_controller)) (Variables|Default|GetMaxDistance))) "Projectile" false 0 "ForDuration" true "(R=1.000000,G=0.000000,B=0.000000,A=1.000000)" "(R=0.000000,G=1.000000,B=0.000000,A=1.000000)" 0.085714))
  (Game|SpawnActorfromClass "/Game/Blueprints/Weapon/BP_Projectile.BP_Projectile_C" (Math|Transform|MakeTransform _returnvalue (select _returnvalue_2 (Math|Conversions|RotationFromXVector (- (.location _outhit) _returnvalue)) (Transformation|GetSocketRotation _mesh "Muzzle")) "0.100000,0.100000,0.100000") "Undefined" 0 0))

(fn ConstructionScript)