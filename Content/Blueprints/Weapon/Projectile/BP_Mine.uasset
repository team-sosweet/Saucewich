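; BP_Mine is a weapon projectile Blueprint for a team-aware mine.
; On activation it caches the team of the TpsCharacter that is its owner's owner.
; On actor overlap it checks whether the other TpsCharacter is on a different team, but that branch is empty, so no detonation or damage happens here.
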(event Collision|EventActorBeginOverlap
  (params (OtherActor :type Actor%20Object%20Reference))
  (bind _astps_character (Utilities|Casting|CastToTpsCharacter OtherActor))
  (if (!= (Class|TpsCharacter|GetTeam _astps_character) (Variables|Default|GetTeam))
    _))

(event EventOnActivated
  (bind _astps_character (Utilities|Casting|CastToTpsCharacter (Components|GetOwner (Components|GetOwner))))
  (Variables|Default|SetTeam (Class|TpsCharacter|GetTeam _astps_character)))

(fn ConstructionScript)