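; BP_GunProjectile is the sauce projectile fired by guns, handling its impact effects when it hits something.
; On hit it plays a random impact sound and spawns a pooled splash particle tinted with the projectile's color.
; It then reads the instigator's SaucewichPlayerState and passes that team, a scale and the hit to an Add call, likely placing team sauce at the impact.
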(event Collision|EventHit
  (params (MyComp :type Primitive%20Component%20Object%20Reference) (Other :type Actor%20Object%20Reference) (OtherComp :type Primitive%20Component%20Object%20Reference) (bSelfMoved :type Boolean) (HitLocation :type Vector :default "0, 0, 0") (HitNormal :type Vector :default "0, 0, 0") (NormalImpulse :type Vector :default "0, 0, 0") (Hit :type Hit%20Result%20Structure%20%28by%20ref%29))
  (Utilities|FlowControl|Sequence
    (:then_0
      (Audio|PlaySoundatLocation (Utilities|Select :Index (Math|Random|RandomInteger 2) :Option%200 "/Game/Assets/Sound/Weapon/sauce_impact1.sauce_impact1" :Option%201 "/Game/Assets/Sound/Weapon/sauce_impact2.sauce_impact2") HitLocation "0, 0, 0" 1.0 1.0 0.0 0 0 0))
    (:then_1
      (bind _returnvalue (Effects|SpawnEmitteratLocation "/Game/Assets/Particles/SauceParticle/PS_SauceImpact.PS_SauceImpact" HitLocation "0, 0, 0" "1.000000,1.000000,1.000000" true "AutoRelease"))
      (Effects|Components|ParticleSystem|SetColorParameter _returnvalue "Color" (Class|Projectile|GetColor)))
    (:then_2
      (bind _assaucewich_player_state (Utilities|Casting|CastToSaucewichPlayerState (Variables|/Script/Engine.Pawn|GetPlayerState (Game|GetInstigator))))
      (Class|SauceMarker|Add (Variables|/Script/Saucewich.SaucewichPlayerState|GetTeam _assaucewich_player_state) 0.5 Hit))))

(fn ConstructionScript)