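; BP_MineProj is a team-owned mine projectile that detonates when an enemy character overlaps it.
; On activation the server takes the owning character's team and zeroes rotation; OnRep_Team applies that team's color.
; Enemy overlap applies damage and spawns a team-colored explosion, then the server releases the mine after a short delay.
; Damage instigated by another team releases it without detonating and awards a MineRemoval score.
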(event Game|Damage|EventAnyDamage
  (params (Damage :type Float%20%28single-precision%29) (DamageType :type Damage%20Type%20Object%20Reference) (InstigatedBy :type Controller%20Object%20Reference) (DamageCauser :type Actor%20Object%20Reference))
  (if (and (> Damage 0.0) (Utilities|IsValid InstigatedBy))
    (bind _assaucewich_player_state (Utilities|Casting|CastToSaucewichPlayerState (Variables|/Script/Engine.Controller|GetPlayerState InstigatedBy)))
    (if (!= (Variables|/Script/Saucewich.SaucewichPlayerState|GetTeam _assaucewich_player_state) (Variables|Default|GetTeam))
      (Class|SaucewichPlayerState|AddScore _assaucewich_player_state "MineRemoval")
      (Class|PoolActor|Release false))))

(event Collision|EventActorBeginOverlap
  (params (OtherActor :type Actor%20Object%20Reference))
  (bind _astps_character (Utilities|Casting|CastToTpsCharacter OtherActor))
  (if (!= (Class|TpsCharacter|GetTeam _astps_character) (Variables|Default|GetTeam))
    (Class|ExplosiveProjectile|ApplyDamage)
    (bind _returnvalue (Effects|SpawnEmitteratLocation "/Game/Assets/Particles/Granade/Granade_Particle.Granade_Particle" (Transformation|GetActorLocation) "0, 0, 0" "0.500000,0.500000,0.500000" true "AutoRelease"))
    (Effects|Components|ParticleSystem|SetColorParameter _returnvalue "Color" (Class|Projectile|GetColor))
    (Networking|SwitchHasAuthority
      (:Authority
        (Utilities|FlowControl|Delay 0.2)
        (Class|PoolActor|Release false)))))

(event EventOnActivated
  (Networking|SwitchHasAuthority
    (:Authority
      (bind _astps_character (Utilities|Casting|CastToTpsCharacter (Components|GetOwner (Components|GetOwner))))
      (Variables|Default|SetTeam (Class|TpsCharacter|GetTeam _astps_character))
      (Transformation|SetActorRotation "0, 0, 0"))))

(fn ConstructionScript)

(fn OnRepTeam
  (bind _assaucewich_game_state (Utilities|Casting|CastToSaucewichGameState (Game|GetGameState)))
  (Class|Projectile|SetColor (.color (Class|SaucewichGameState|GetTeamData _assaucewich_game_state (Variables|Default|GetTeam)))))