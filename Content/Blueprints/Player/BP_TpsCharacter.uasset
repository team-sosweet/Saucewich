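; Third-person player character for the sandwich-making mode, with touch look controls, a widget-component HUD and perk-based stat bonuses.
; Outside dedicated servers, BeginPlay binds the HUD's ingredient display to the PlayerState, awaited by a Delay-loop macro that polls until valid.
; Tick turns touch drags into sensitivity-scaled look input and shrinks the widget with distance from the local pawn.
; GetSpeedRatio and GetArmor add Olive and Cheese perk bonuses respectively.
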(event Custom|Set%20Widget%20Size
  (bind _returnvalue (Transformation|GetActorLocation))
  (bind _local_pawn (Variables|Default|GetLocal%20Pawn))
  (bind _returnvalue_2 (Transformation|GetActorLocation _local_pawn))
  (bind _returnvalue_3 (Math|Vector|Distance(Vector) _returnvalue _returnvalue_2))
  (bind _returnvalue_4 (Math|Float|MapRangeClamped _returnvalue_3 0.0 2e+03 2.6e+02 8e+01))
  (Class|WidgetComponent|SetDrawSize (Variables|Default|GetWidget) (Math|Vector2D|MakeVector2D _returnvalue_4 _returnvalue_4)))

(event Custom|Mobile%20Rotation
  (bind _returnvalue (Game|GetPlayerController 0))
  (bind _touch_index (Variables|Default|GetTouch%20Index))
  (bind (_locationx _locationy _biscurrentlypressed) (Class|PlayerController|GetInputTouchState _returnvalue _touch_index))
  (if (Pawn|IsLocallyControlled)
    (if _biscurrentlypressed
      (if (Variables|Default|GetWas%20Touched)
        (Pawn|Input|AddControllerYawInput (.x (* (- (Math|Vector2D|MakeVector2D _locationx _locationy) (Variables|Default|GetTouch%20Pos)) (Class|SaucewichGameInstance|GetSensitivity (Variables|Default|GetGame%20Instance)))))
        (Pawn|Input|AddControllerPitchInput (.y (* (- (Math|Vector2D|MakeVector2D _locationx _locationy) (Variables|Default|GetTouch%20Pos)) (Class|SaucewichGameInstance|GetSensitivity (Variables|Default|GetGame%20Instance)))))
        (else
          (Variables|Default|SetWas%20Touched true)))
      (Variables|Default|SetTouch%20Pos (Math|Vector2D|MakeVector2D _locationx _locationy))
      (else
        (Variables|Default|SetWas%20Touched false)))))

(event EventTick
  (params (DeltaSeconds :type Float%20%28single-precision%29))
  (if (not (and (Networking|IsServer) (Networking|IsDedicatedServer)))
    (CallFunction|MobileRotation)
    (CallFunction|SetWidgetSize)))

(event EventBeginPlay
  (if (not (and (Networking|IsServer) (Networking|IsDedicatedServer)))
    (bind _assaucewich_game_instance (Utilities|Casting|CastToSaucewichGameInstance (Game|GetGameInstance)))
    (Variables|Default|SetGame%20Instance _assaucewich_game_instance)
    (Variables|Default|SetLocal%20Pawn (Pawn|GetControlledPawn (Game|GetPlayerController 0)))
    (bind _asumg_user_hud (Utilities|Casting|CastToUMG_UserHUD (UserInterface|GetUserWidgetObject (Variables|Default|GetWidget))))
    (Class|UserHUD|Init _asumg_user_hud self)
    (Class|BaseWidget|SetComponent _asumg_user_hud "/Game/Blueprints/Widget/HUD/UMG_MakeSandwichHUDComponent.UMG_MakeSandwichHUDComponent_C")
    (bind _asumg_make_sandwich_hudcomponent (Utilities|Casting|CastToUMG_MakeSandwichHUDComponent (Variables|/Script/Saucewich.BaseWidget|GetComponent _asumg_user_hud)))
    (bind _player_state (Utilities|GetPlayerState)
      (:%20%20
        (bind _asmake_sandwich_player_state (Utilities|Casting|CastToMakeSandwichPlayerState _player_state))
        (Variables|/Game/Blueprints/Widget/HUD/UMG_HUDIngredient.UMG_HUDIngredient_C|SetPlayer%20State (Variables|/Game/Blueprints/Widget/HUD/UMG_MakeSandwichHUDComponent.UMG_MakeSandwichHUDComponent_C|GetIngredient _asumg_make_sandwich_hudcomponent) _asmake_sandwich_player_state)))
    (else
      (Components|Activation|Deactivate (Variables|Default|GetWidget)))))

(event Input|TouchEvents|InputTouch
  (params (Location :type Vector) (FingerIndex :type ETouchIndex%20Enum))
  (:Pressed
    (Default|CallOnPressedTouch))
  (:Released
    (Default|CallOnReleasedTouch))
  (:Moved
    (Variables|Default|SetTouch%20Index FingerIndex)))

(fn ConstructionScript)

(fn GetSpeedRatio
  (bind _returnvalue (|CallParentFunction))
  (return (select (Class|TpsCharacter|HasPerk "/Game/Blueprints/GameMode/MakeSandwich/Entity/Perk/BP_Olive.BP_Olive_C") (+ _returnvalue 0.2) _returnvalue)))

(fn GetArmor
  (return (select (Class|TpsCharacter|HasPerk "/Game/Blueprints/GameMode/MakeSandwich/Entity/Perk/BP_Cheese.BP_Cheese_C") (+ 0.0 0.2) 0.0) 0.0))