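; BP_TransitionHUD is the HUD for a transition level that shows a description screen and moves on to the next map.
; BeginPlay calls InitHUD with a hardcoded MakeSandwich mode, which selects an image from the DescriptionImages map for a UMG_Transition widget.
; Right after adding the widget to the viewport, it opens the level named by the NextMap option in the game mode's options string.
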(event Custom|Init%20HUD
  (params (Mode :type EGameRule%20Enum :default "Lobby"))
  (bind _returnvalue (UserInterface|CreateWidget "/Game/Blueprints/Widget/Transition/UMG_Transition.UMG_Transition_C" (Variables|Default|GetPlayerOwner) (.Value (Utilities|Map|Find (Variables|Default|GetDescription%20Images) Mode))))
  (UserInterface|Viewport|AddtoViewport _returnvalue 0)
  (Game|OpenLevel(byName) (Utilities|String|StringToName (Class|GameplayStatics|ParseOption (Variables|/Script/Engine.GameModeBase|GetOptionsString (Game|GetGameMode)) "NextMap"))))

(event EventBeginPlay
  (CallFunction|InitHUD "MakeSandwich"))

(fn ConstructionScript)